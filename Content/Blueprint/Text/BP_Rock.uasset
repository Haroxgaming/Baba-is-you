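; BP_Rock is an interactable rock that the player shoves away from themselves in fixed steps.
; BeginPlay caches the player's BP_ThirdPersonCharacter, and Interact compares its world position with the rock's to pick a direction along a world axis.
; X is tested first, so Y moves only happen when both X values match exactly.
; Each push is an instant SetActorLocation offset, with no interpolation.
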(event EventBeginPlay
  (bind _asbp_third_person_character (Utilities|Casting|CastToBP_ThirdPersonCharacter (Game|GetPlayerCharacter 0)))
  (Variables|Default|SetPlayer%20ref _asbp_third_person_character))

(event EventInteract
  (bind _returnvalue (Transformation|GetActorLocation))
  (bind _returnvalue_2 (Transformation|GetActorLocation))
  (bind _player_ref (Variables|Default|GetPlayer%20ref))
  (bind _player_ref_2 (Variables|Default|GetPlayer%20ref))
  (bind _returnvalue_3 (Transformation|GetActorLocation _player_ref_2))
  (bind _returnvalue_4 (Transformation|GetActorLocation _player_ref))
  (if (> (.x _returnvalue_3) (.x _returnvalue))
    (Transformation|SetActorLocation (Math|Vector|MakeVector (+ (.x _returnvalue) -1e+02) (.y _returnvalue) (.z _returnvalue)) false false)
    (elif (< (.x _returnvalue_3) (.x _returnvalue))
      (Transformation|SetActorLocation (Math|Vector|MakeVector (+ (.x _returnvalue) 1e+02) (.y _returnvalue) (.z _returnvalue)) false false)
      (elif (< (.y _returnvalue_4) (.y _returnvalue_2))
        (Transformation|SetActorLocation (Math|Vector|MakeVector (.x _returnvalue_2) (+ (.y _returnvalue_2) 1e+02) (.z _returnvalue_2)) false false)
        (elif (> (.y _returnvalue_4) (.y _returnvalue_2))
          (Transformation|SetActorLocation (Math|Vector|MakeVector (.x _returnvalue_2) (+ (.y _returnvalue_2) -1e+02) (.z _returnvalue_2)) false false))))))

(fn ConstructionScript)