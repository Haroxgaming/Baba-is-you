(event Custom|Check
  (bind _returnvalue (Transformation|GetActorLocation))
  (bind _returnvalue_2 (Transformation|GetActorLocation))
  (bind _returnvalue_3 (Transformation|GetActorLocation))
  (bind _returnvalue_4 (Transformation|GetActorLocation))
  (bind _returnvalue_5 (Transformation|GetActorLocation))
  (bind _returnvalue_6 (Transformation|GetActorLocation))
  (bind _game_ref (Variables|Default|Getgame%20ref))
  (bind _game_ref_2 (Variables|Default|Getgame%20ref))
  (bind _game_ref_3 (Variables|Default|Getgame%20ref))
  (bind _game_ref_4 (Variables|Default|Getgame%20ref))
  (bind _game_ref_5 (Variables|Default|Getgame%20ref))
  (bind _game_ref_6 (Variables|Default|Getgame%20ref))
  (bind _game_ref_7 (Variables|Default|Getgame%20ref))
  (bind _game_ref_8 (Variables|Default|Getgame%20ref))
  (bind _game_ref_9 (Variables|Default|Getgame%20ref))
  (bind _game_ref_10 (Variables|Default|Getgame%20ref))
  (bind _game_ref_11 (Variables|Default|Getgame%20ref))
  (bind _returnvalue_7 (+ (.y _returnvalue_5) -1e+02))
  (bind (_outhit _returnvalue_8) (Collision|LineTraceByChannel (Transformation|GetActorLocation) (Math|Vector|MakeVector (.x _returnvalue_3) (+ (.y _returnvalue_3) 1e+02) (.z _returnvalue_3)) "TraceTypeQuery1" false 0 "ForDuration"))
  (if _returnvalue_8
    (if (== (.hitactor _outhit) (Variables|Default|GetWin%20ref))
      (Variables|/Game/Blueprint/Text/BP_Game.BP_Game_C|SetWin (Variables|Default|Getgame%20ref) true)
      (bind _outhit_2 (Collision|LineTraceByChannel (Transformation|GetActorLocation) (Math|Vector|MakeVector (.x _returnvalue) (+ (.y _returnvalue) -1e+02) (.z _returnvalue)) "TraceTypeQuery1" false 0 "ForDuration"))
      (if (== (.hitactor _outhit_2) (Variables|Default|GetRock%20ref))
        (Variables|/Game/Blueprint/Text/BP_Game.BP_Game_C|SetRock _game_ref_9 true)
        (else
          (Variables|/Game/Blueprint/Text/BP_Game.BP_Game_C|SetRock _game_ref_9 false)
          (if (== (.hitactor _outhit_2) (Variables|Default|GetPush%20ref))
            (Variables|/Game/Blueprint/Text/BP_Game.BP_Game_C|SetPush _game_ref_9 true)
            (else
              (Variables|/Game/Blueprint/Text/BP_Game.BP_Game_C|SetPush _game_ref_9 false)
              (if (== (.hitactor _outhit_2) (Variables|Default|Getdefeat%20ref))
                (Variables|/Game/Blueprint/Text/BP_Game.BP_Game_C|SetDefeat _game_ref_9 true)
                (else
                  (Variables|/Game/Blueprint/Text/BP_Game.BP_Game_C|SetDefeat _game_ref_9 false)
                  (if (== (.hitactor _outhit_2) (Variables|Default|GetWall%20ref))
                    (Variables|/Game/Blueprint/Text/BP_Game.BP_Game_C|SetWall _game_ref_9 true)
                    (else
                      (Variables|/Game/Blueprint/Text/BP_Game.BP_Game_C|SetWall _game_ref_9 false)
                      (if (== (.hitactor _outhit_2) (Variables|Default|GetFlag%20ref))
                        (Variables|/Game/Blueprint/Text/BP_Game.BP_Game_C|SetFlag _game_ref_9 true)
                        (else
                          (Variables|/Game/Blueprint/Text/BP_Game.BP_Game_C|SetFlag _game_ref_9 false)))))))))))
      (else
        (Variables|/Game/Blueprint/Text/BP_Game.BP_Game_C|SetWin (Variables|Default|Getgame%20ref) false)
        (if (== (.hitactor _outhit) (Variables|Default|GetPush%20ref))
          (Variables|/Game/Blueprint/Text/BP_Game.BP_Game_C|SetPush (Variables|Default|Getgame%20ref) true)
          (bind _outhit_3 (Collision|LineTraceByChannel (Transformation|GetActorLocation) (Math|Vector|MakeVector (.x _returnvalue_2) (+ (.y _returnvalue_2) -1e+02) (.z _returnvalue_2)) "TraceTypeQuery1" false 0 "ForDuration"))
          (if (== (.hitactor _outhit_3) (Variables|Default|GetRock%20ref))
            (Variables|/Game/Blueprint/Text/BP_Game.BP_Game_C|SetRock _game_ref true)
            (else
              (Variables|/Game/Blueprint/Text/BP_Game.BP_Game_C|SetRock _game_ref false)
              (if (== (.hitactor _outhit_3) (Variables|Default|GetWin%20ref))
                (Variables|/Game/Blueprint/Text/BP_Game.BP_Game_C|SetWin _game_ref true)
                (else
                  (Variables|/Game/Blueprint/Text/BP_Game.BP_Game_C|SetWin _game_ref false)
                  (if (== (.hitactor _outhit_3) (Variables|Default|Getdefeat%20ref))
                    (Variables|/Game/Blueprint/Text/BP_Game.BP_Game_C|SetDefeat _game_ref true)
                    (else
                      (Variables|/Game/Blueprint/Text/BP_Game.BP_Game_C|SetDefeat _game_ref false)
                      (if (== (.hitactor _outhit_3) (Variables|Default|GetWall%20ref))
                        (Variables|/Game/Blueprint/Text/BP_Game.BP_Game_C|SetWall _game_ref true)
                        (else
                          (Variables|/Game/Blueprint/Text/BP_Game.BP_Game_C|SetWall _game_ref false)
                          (if (== (.hitactor _outhit_3) (Variables|Default|GetFlag%20ref))
                            (Variables|/Game/Blueprint/Text/BP_Game.BP_Game_C|SetFlag _game_ref true)
                            (else
                              (Variables|/Game/Blueprint/Text/BP_Game.BP_Game_C|SetFlag _game_ref false)))))))))))
          (else
            (Variables|/Game/Blueprint/Text/BP_Game.BP_Game_C|SetPush _game_ref_11 false)
            (if (== (.hitactor _outhit) (Variables|Default|Getdefeat%20ref))
              (Variables|/Game/Blueprint/Text/BP_Game.BP_Game_C|SetDefeat _game_ref_11 true)
              (bind _outhit_4 (Collision|LineTraceByChannel (Transformation|GetActorLocation) (Math|Vector|MakeVector (.x _returnvalue_4) (+ (.y _returnvalue_4) -1e+02) (.z _returnvalue_4)) "TraceTypeQuery1" false 0 "ForDuration"))
              (if (== (.hitactor _outhit_4) (Variables|Default|GetRock%20ref))
                (Variables|/Game/Blueprint/Text/BP_Game.BP_Game_C|SetRock _game_ref_3 true)
                (else
                  (Variables|/Game/Blueprint/Text/BP_Game.BP_Game_C|SetRock _game_ref_3 false)
                  (if (== (.hitactor _outhit_4) (Variables|Default|GetWin%20ref))
                    (Variables|/Game/Blueprint/Text/BP_Game.BP_Game_C|SetWin _game_ref_3 true)
                    (else
                      (Variables|/Game/Blueprint/Text/BP_Game.BP_Game_C|SetWin _game_ref_3 false)
                      (if (== (.hitactor _outhit_4) (Variables|Default|GetPush%20ref))
                        (Variables|/Game/Blueprint/Text/BP_Game.BP_Game_C|SetPush _game_ref_3 true)
                        (else
                          (Variables|/Game/Blueprint/Text/BP_Game.BP_Game_C|SetPush _game_ref_3 false)
                          (if (== (.hitactor _outhit_4) (Variables|Default|GetWall%20ref))
                            (Variables|/Game/Blueprint/Text/BP_Game.BP_Game_C|SetWall _game_ref_3 true)
                            (else
                              (Variables|/Game/Blueprint/Text/BP_Game.BP_Game_C|SetWall _game_ref_3 false)
                              (if (== (.hitactor _outhit_4) (Variables|Default|GetFlag%20ref))
                                (Variables|/Game/Blueprint/Text/BP_Game.BP_Game_C|SetFlag _game_ref_3 true)
                                (else
                                  (Variables|/Game/Blueprint/Text/BP_Game.BP_Game_C|SetFlag _game_ref_3 false)))))))))))
              (else
                (Variables|/Game/Blueprint/Text/BP_Game.BP_Game_C|SetDefeat _game_ref_10 false)
                (if (== (.hitactor _outhit) (Variables|Default|GetRock%20ref))
                  (Variables|/Game/Blueprint/Text/BP_Game.BP_Game_C|SetRock _game_ref_10 true)
                  (bind _outhit_5 (Collision|LineTraceByChannel _returnvalue_6 (Math|Vector|MakeVector (.x _returnvalue_5) _returnvalue_7 (.z _returnvalue_5)) "TraceTypeQuery1" false 0 "ForDuration"))
                  (if (== (.hitactor _outhit_5) (Variables|Default|GetWin%20ref))
                    (Variables|/Game/Blueprint/Text/BP_Game.BP_Game_C|SetWin _game_ref_8 true)
                    (else
                      (Variables|/Game/Blueprint/Text/BP_Game.BP_Game_C|SetWin _game_ref_8 false)
                      (if (== (.hitactor _outhit_5) (Variables|Default|GetPush%20ref))
                        (Variables|/Game/Blueprint/Text/BP_Game.BP_Game_C|SetPush _game_ref_8 true)
                        (else
                          (Variables|/Game/Blueprint/Text/BP_Game.BP_Game_C|SetPush _game_ref_8 false)
                          (if (== (.hitactor _outhit_5) (Variables|Default|Getdefeat%20ref))
                            (Variables|/Game/Blueprint/Text/BP_Game.BP_Game_C|SetDefeat _game_ref_8 true)
                            (else
                              (Variables|/Game/Blueprint/Text/BP_Game.BP_Game_C|SetDefeat _game_ref_8 false)
                              (if (== (.hitactor _outhit_5) (Variables|Default|GetWall%20ref))
                                (Variables|/Game/Blueprint/Text/BP_Game.BP_Game_C|SetWall _game_ref_8 true)
                                (else
                                  (Variables|/Game/Blueprint/Text/BP_Game.BP_Game_C|SetWall _game_ref_8 false)
                                  (if (== (.hitactor _outhit_5) (Variables|Default|GetFlag%20ref))
                                    (Variables|/Game/Blueprint/Text/BP_Game.BP_Game_C|SetFlag _game_ref_8 true)
                                    (else
                                      (Variables|/Game/Blueprint/Text/BP_Game.BP_Game_C|SetFlag _game_ref_8 false)))))))))))
                  (else
                    (Variables|/Game/Blueprint/Text/BP_Game.BP_Game_C|SetRock _game_ref_6 false)
                    (if (== (.hitactor _outhit) (Variables|Default|GetWall%20ref))
                      (Variables|/Game/Blueprint/Text/BP_Game.BP_Game_C|SetWall _game_ref_6 true)
                      (bind _outhit_6 (Collision|LineTraceByChannel _returnvalue_6 (Math|Vector|MakeVector (.x _returnvalue_5) _returnvalue_7 (.z _returnvalue_5)) "TraceTypeQuery1" false 0 "ForDuration"))
                      (if (== (.hitactor _outhit_6) (Variables|Default|GetWin%20ref))
                        (Variables|/Game/Blueprint/Text/BP_Game.BP_Game_C|SetWin _game_ref_7 true)
                        (else
                          (Variables|/Game/Blueprint/Text/BP_Game.BP_Game_C|SetWin _game_ref_7 false)
                          (if (== (.hitactor _outhit_6) (Variables|Default|GetPush%20ref))
                            (Variables|/Game/Blueprint/Text/BP_Game.BP_Game_C|SetPush _game_ref_7 true)
                            (else
                              (Variables|/Game/Blueprint/Text/BP_Game.BP_Game_C|SetPush _game_ref_7 false)
                              (if (== (.hitactor _outhit_6) (Variables|Default|Getdefeat%20ref))
                                (Variables|/Game/Blueprint/Text/BP_Game.BP_Game_C|SetDefeat _game_ref_7 true)
                                (else
                                  (Variables|/Game/Blueprint/Text/BP_Game.BP_Game_C|SetDefeat _game_ref_7 false)
                                  (if (== (.hitactor _outhit_6) (Variables|Default|GetRock%20ref))
                                    (Variables|/Game/Blueprint/Text/BP_Game.BP_Game_C|SetRock _game_ref_7 true)
                                    (else
                                      (Variables|/Game/Blueprint/Text/BP_Game.BP_Game_C|SetRock _game_ref_7 false)
                                      (if (== (.hitactor _outhit_6) (Variables|Default|GetFlag%20ref))
                                        (Variables|/Game/Blueprint/Text/BP_Game.BP_Game_C|SetFlag _game_ref_7 true)
                                        (else
                                          (Variables|/Game/Blueprint/Text/BP_Game.BP_Game_C|SetFlag _game_ref_7 false)))))))))))
                      (else
                        (Variables|/Game/Blueprint/Text/BP_Game.BP_Game_C|SetWall _game_ref_5 false)
                        (if (== (.hitactor _outhit) (Variables|Default|GetFlag%20ref))
                          (Variables|/Game/Blueprint/Text/BP_Game.BP_Game_C|SetFlag _game_ref_5 true)
                          (bind _outhit_7 (Collision|LineTraceByChannel _returnvalue_6 (Math|Vector|MakeVector (.x _returnvalue_5) _returnvalue_7 (.z _returnvalue_5)) "TraceTypeQuery1" false 0 "ForDuration"))
                          (if (== (.hitactor _outhit_7) (Variables|Default|GetWin%20ref))
                            (Variables|/Game/Blueprint/Text/BP_Game.BP_Game_C|SetWin _game_ref_4 true)
                            (else
                              (Variables|/Game/Blueprint/Text/BP_Game.BP_Game_C|SetWin _game_ref_4 false)
                              (if (== (.hitactor _outhit_7) (Variables|Default|GetPush%20ref))
                                (Variables|/Game/Blueprint/Text/BP_Game.BP_Game_C|SetPush _game_ref_4 true)
                                (else
                                  (Variables|/Game/Blueprint/Text/BP_Game.BP_Game_C|SetPush _game_ref_4 false)
                                  (if (== (.hitactor _outhit_7) (Variables|Default|Getdefeat%20ref))
                                    (Variables|/Game/Blueprint/Text/BP_Game.BP_Game_C|SetDefeat _game_ref_4 true)
                                    (else
                                      (Variables|/Game/Blueprint/Text/BP_Game.BP_Game_C|SetDefeat _game_ref_4 false)
                                      (if (== (.hitactor _outhit_7) (Variables|Default|GetRock%20ref))
                                        (Variables|/Game/Blueprint/Text/BP_Game.BP_Game_C|SetRock _game_ref_4 true)
                                        (else
                                          (Variables|/Game/Blueprint/Text/BP_Game.BP_Game_C|SetRock _game_ref_4 false)
                                          (if (== (.hitactor _outhit_7) (Variables|Default|GetWall%20ref))
                                            (Variables|/Game/Blueprint/Text/BP_Game.BP_Game_C|SetWall _game_ref_4 true)
                                            (else
                                              (Variables|/Game/Blueprint/Text/BP_Game.BP_Game_C|SetWall _game_ref_4 false)))))))))))
                          (else
                            (Variables|/Game/Blueprint/Text/BP_Game.BP_Game_C|SetFlag _game_ref_5 false)
                            (Variables|/Game/Blueprint/Text/BP_Game.BP_Game_C|SetWin _game_ref_5 false)))))))))))))
    (else
      (Variables|/Game/Blueprint/Text/BP_Game.BP_Game_C|SetPush _game_ref_2 false)
      (Variables|/Game/Blueprint/Text/BP_Game.BP_Game_C|SetDefeat _game_ref_2 false)
      (Variables|/Game/Blueprint/Text/BP_Game.BP_Game_C|SetRock _game_ref_2 false)
      (Variables|/Game/Blueprint/Text/BP_Game.BP_Game_C|SetWall _game_ref_2 false)
      (Variables|/Game/Blueprint/Text/BP_Game.BP_Game_C|SetFlag _game_ref_2 false)
      (Variables|/Game/Blueprint/Text/BP_Game.BP_Game_C|SetWin _game_ref_2 false))))

(event EventBeginPlay
  (bind _asbp_third_person_character (Utilities|Casting|CastToBP_ThirdPersonCharacter (Game|GetPlayerCharacter 0)))
  (Variables|Default|SetPlayer%20ref _asbp_third_person_character)
  (bind _returnvalue (Actor|GetActorOfClass "/Game/Blueprint/Text/BP_Win.BP_Win_C"))
  (Variables|Default|SetWin%20ref _returnvalue)
  (bind _returnvalue_2 (Actor|GetActorOfClass "/Game/Blueprint/Text/BP_Push.BP_Push_C"))
  (Variables|Default|SetPush%20ref _returnvalue_2)
  (bind _returnvalue_3 (Actor|GetActorOfClass "/Game/Blueprint/Text/BP_Defeat.BP_Defeat_C"))
  (Variables|Default|Setdefeat%20ref _returnvalue_3)
  (bind _returnvalue_4 (Actor|GetActorOfClass "/Game/Blueprint/Text/BP_Flag.BP_Flag_C"))
  (Variables|Default|SetFlag%20ref _returnvalue_4)
  (bind _returnvalue_5 (Actor|GetActorOfClass "/Game/Blueprint/Text/BP_Rock.BP_Rock_C"))
  (Variables|Default|SetRock%20ref _returnvalue_5)
  (bind _returnvalue_6 (Actor|GetActorOfClass "/Game/Blueprint/Text/BP_Wall.BP_Wall_C"))
  (Variables|Default|SetWall%20ref _returnvalue_6)
  (bind _returnvalue_7 (Actor|GetActorOfClass "/Game/Blueprint/Text/BP_Game.BP_Game_C"))
  (Variables|Default|Setgame%20ref _returnvalue_7))

(event EventInteract
  (bind _returnvalue (Transformation|GetActorLocation))
  (bind _returnvalue_2 (Transformation|GetActorLocation))
  (bind _player_ref (Variables|Default|GetPlayer%20ref))
  (bind _player_ref_2 (Variables|Default|GetPlayer%20ref))
  (bind _returnvalue_3 (Transformation|GetActorLocation _player_ref_2))
  (bind _returnvalue_4 (Transformation|GetActorLocation _player_ref))
  (if (> (.x _returnvalue_3) (.x _returnvalue))
    (Transformation|SetActorLocation (Math|Vector|MakeVector (+ (.x _returnvalue) -1e+02) (.y _returnvalue) (.z _returnvalue)) false false)
    (elif (< (.x _returnvalue_3) (.x _returnvalue))
      (Transformation|SetActorLocation (Math|Vector|MakeVector (+ (.x _returnvalue) 1e+02) (.y _returnvalue) (.z _returnvalue)) false false)
      (elif (< (.y _returnvalue_4) (.y _returnvalue_2))
        (Transformation|SetActorLocation (Math|Vector|MakeVector (.x _returnvalue_2) (+ (.y _returnvalue_2) 1e+02) (.z _returnvalue_2)) false false)
        (elif (> (.y _returnvalue_4) (.y _returnvalue_2))
          (Transformation|SetActorLocation (Math|Vector|MakeVector (.x _returnvalue_2) (+ (.y _returnvalue_2) -1e+02) (.z _returnvalue_2)) false false))))))

(fn ConstructionScript)