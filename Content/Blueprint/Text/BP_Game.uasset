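; BP_Game is the rule manager for a word-rule puzzle, applying Win, Push, Defeat and object-swap rules to single Flag, Rock and Wall actors.
; On BeginPlay it caches those actors and BP_IS, then starts a looping timer.
; Each tick calls BP_IS's Check, then walks a prioritized branch tree over its own rule booleans, handling only the first active noun.
; Branches set the object's state flags or replace it by spawning another class and destroying it.
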(event Custom|Check
  (bind _flagobject_ref (Variables|Default|GetFlagObject%20ref))
  (bind _flagobject_ref_2 (Variables|Default|GetFlagObject%20ref))
  (bind _flagobject_ref_3 (Variables|Default|GetFlagObject%20ref))
  (bind _flagobject_ref_4 (Variables|Default|GetFlagObject%20ref))
  (bind _flagobject_ref_5 (Variables|Default|GetFlagObject%20ref))
  (bind _flagobject_ref_6 (Variables|Default|GetFlagObject%20ref))
  (bind _rockobject_ref (Variables|Default|GetRockObject%20ref))
  (bind _rockobject_ref_2 (Variables|Default|GetRockObject%20ref))
  (bind _rockobject_ref_3 (Variables|Default|GetRockObject%20ref))
  (bind _rockobject_ref_4 (Variables|Default|GetRockObject%20ref))
  (bind _rockobject_ref_5 (Variables|Default|GetRockObject%20ref))
  (bind _wallobject_ref (Variables|Default|GetWallObject%20ref))
  (bind _wallobject_ref_2 (Variables|Default|GetWallObject%20ref))
  (bind _wallobject_ref_3 (Variables|Default|GetWallObject%20ref))
  (bind _wallobject_ref_4 (Variables|Default|GetWallObject%20ref))
  (bind _wallobject_ref_5 (Variables|Default|GetWallObject%20ref))
  (bind _flagobject_ref_7 (Variables|Default|GetFlagObject%20ref))
  (Variables|/Game/Blueprint/Object/BP_FlagObject.BP_FlagObject_C|SetWin _flagobject_ref_2 false)
  (Default|Check (Variables|Default|GetIs%20ref))
  (if (Variables|Default|GetFlag)
    (if (Variables|Default|GetWin)
      (Variables|/Game/Blueprint/Object/BP_FlagObject.BP_FlagObject_C|SetWin _flagobject_ref true)
      (else
        (Variables|/Game/Blueprint/Object/BP_FlagObject.BP_FlagObject_C|SetWin _flagobject_ref false)
        (if (Variables|Default|GetPush)
          (Variables|/Game/Blueprint/Object/BP_FlagObject.BP_FlagObject_C|SetCan%20Push _flagobject_ref_3 true)
          (else
            (Variables|/Game/Blueprint/Object/BP_FlagObject.BP_FlagObject_C|SetCan%20Push _flagobject_ref_3 false)
            (if (Variables|Default|GetDefeat)
              (Variables|/Game/Blueprint/Object/BP_FlagObject.BP_FlagObject_C|SetDeath _flagobject_ref_4 true)
              (else
                (Variables|/Game/Blueprint/Object/BP_FlagObject.BP_FlagObject_C|SetDeath _flagobject_ref_4 false)
                (if (Variables|Default|GetRock)
                  (Game|SpawnActorfromClass "/Game/Blueprint/Text/BP_Rock.BP_Rock_C" (Transformation|GetActorTransform _flagobject_ref_5) "Undefined" "MultiplyWithRoot" _flagobject_ref_5 0)
                  (Actor|DestroyActor (Variables|Default|GetFlagObject%20ref))
                  (elif (Variables|Default|GetWall)
                    (Game|SpawnActorfromClass "/Game/Blueprint/Text/BP_Wall.BP_Wall_C" (Transformation|GetActorTransform _flagobject_ref_6) "Undefined" "MultiplyWithRoot" _flagobject_ref_6 0)
                    (Actor|DestroyActor (Variables|Default|GetFlagObject%20ref))))))))))
    (else
      (Collision|SetCollisionEnabled (Variables|/Game/Blueprint/Object/BP_FlagObject.BP_FlagObject_C|GetStaticMesh _flagobject_ref_2) "NoCollision")
      (Variables|/Game/Blueprint/Object/BP_FlagObject.BP_FlagObject_C|SetDeath _flagobject_ref_7 false)
      (Variables|/Game/Blueprint/Object/BP_FlagObject.BP_FlagObject_C|SetCan%20Push _flagobject_ref_7 false)
      (Variables|/Game/Blueprint/Object/BP_FlagObject.BP_FlagObject_C|SetWin _flagobject_ref_7 false)
      (if (Variables|Default|GetRock)
        (if (Variables|Default|GetWin)
          (Variables|/Game/Blueprint/Object/BP_RockObject.BP_RockObject_C|SetWin _rockobject_ref_4 true)
          (else
            (Variables|/Game/Blueprint/Object/BP_RockObject.BP_RockObject_C|SetWin _rockobject_ref_4 false)
            (if (Variables|Default|GetPush)
              (Variables|/Game/Blueprint/Object/BP_RockObject.BP_RockObject_C|SetCan%20Push _rockobject_ref_5 true)
              (else
                (Variables|/Game/Blueprint/Object/BP_RockObject.BP_RockObject_C|SetCan%20Push _rockobject_ref_5 false)
                (if (Variables|Default|GetDefeat)
                  (Variables|/Game/Blueprint/Object/BP_RockObject.BP_RockObject_C|SetDeath _rockobject_ref true)
                  (else
                    (Variables|/Game/Blueprint/Object/BP_RockObject.BP_RockObject_C|SetDeath _rockobject_ref false)
                    (if (Variables|Default|GetFlag)
                      (Game|SpawnActorfromClass "/Game/Blueprint/Object/BP_FlagObject.BP_FlagObject_C" (Transformation|GetActorTransform _rockobject_ref_2) "Undefined" "MultiplyWithRoot" _rockobject_ref_2 0)
                      (Actor|DestroyActor (Variables|Default|GetRockObject%20ref))
                      (elif (Variables|Default|GetWall)
                        (Game|SpawnActorfromClass "/Game/Blueprint/Text/BP_Wall.BP_Wall_C" (Transformation|GetActorTransform _rockobject_ref_3) "Undefined" "MultiplyWithRoot" _rockobject_ref_3 0)
                        (Actor|DestroyActor (Variables|Default|GetRockObject%20ref))))))))))
        (elif (Variables|Default|GetWall)
          (if (Variables|Default|GetWin)
            (Variables|/Game/Blueprint/Object/BP_WallObject.BP_WallObject_C|SetWin _wallobject_ref false)
            (else
              (Variables|/Game/Blueprint/Object/BP_WallObject.BP_WallObject_C|SetWin _wallobject_ref false)
              (if (Variables|Default|GetPush)
                (Variables|/Game/Blueprint/Object/BP_WallObject.BP_WallObject_C|SetCan%20Push _wallobject_ref_2 true)
                (else
                  (Variables|/Game/Blueprint/Object/BP_WallObject.BP_WallObject_C|SetCan%20Push _wallobject_ref_2 false)
                  (if (Variables|Default|GetDefeat)
                    (Variables|/Game/Blueprint/Object/BP_WallObject.BP_WallObject_C|SetDeath _wallobject_ref_3 true)
                    (else
                      (Variables|/Game/Blueprint/Object/BP_WallObject.BP_WallObject_C|SetDeath _wallobject_ref_3 false)
                      (if (Variables|Default|GetFlag)
                        (Game|SpawnActorfromClass "/Game/Blueprint/Object/BP_FlagObject.BP_FlagObject_C" (Transformation|GetActorTransform _wallobject_ref_4) "Undefined" "MultiplyWithRoot" _wallobject_ref_4 0)
                        (Actor|DestroyActor _wallobject_ref_4)
                        (elif (Variables|Default|GetRock)
                          (Game|SpawnActorfromClass "/Game/Blueprint/Object/BP_RockObject.BP_RockObject_C" (Transformation|GetActorTransform _wallobject_ref_5) "Undefined" "MultiplyWithRoot" _wallobject_ref_5 0)
                          (Actor|DestroyActor _wallobject_ref_5))))))))))))))

(event EventBeginPlay
  (bind _returnvalue (Actor|GetActorOfClass "/Game/Blueprint/Text/BP_IS.BP_IS_C"))
  (Variables|Default|SetIs%20ref _returnvalue)
  (bind _returnvalue_2 (Actor|GetActorOfClass "/Game/Blueprint/Object/BP_FlagObject.BP_FlagObject_C"))
  (Variables|Default|SetFlagObject%20ref _returnvalue_2)
  (bind _returnvalue_3 (Actor|GetActorOfClass "/Game/Blueprint/Object/BP_WallObject.BP_WallObject_C"))
  (Variables|Default|SetWallObject%20ref _returnvalue_3)
  (bind _returnvalue_4 (Actor|GetActorOfClass "/Game/Blueprint/Object/BP_RockObject.BP_RockObject_C"))
  (Variables|Default|SetRockObject%20ref _returnvalue_4)
  (Utilities|Time|SetTimerbyEvent (delegate Custom|Check) 1.0 true))

(fn ConstructionScript)