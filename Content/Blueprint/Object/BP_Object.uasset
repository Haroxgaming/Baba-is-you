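; BP_Object is a configurable world object that takes the form of a wall, rock, flag, key or door.
; The construction script switches on ChooseMesh to set the static mesh, its scale and a local offset.
; Only the Wall case also assigns a material, a beveled clay brick.
; The event graph has no active logic, so the Blueprint handles appearance only.
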(event EventBeginPlay)

(fn ConstructionScript
  (bind _staticmesh (Variables|Default|GetStaticMesh))
  (bind _staticmesh_2 (Variables|Default|GetStaticMesh))
  (bind _staticmesh_3 (Variables|Default|GetStaticMesh))
  (switch Utilities|FlowControl|Switch|SwitchonE_Object (Variables|Default|GetChoose%20mesh)
    (:NewEnumerator0
      (Components|StaticMesh|SetStaticMesh _staticmesh "/Game/StarterContent/Shapes/Shape_Cube.Shape_Cube")
      (Rendering|Material|SetMaterial _staticmesh 0 "/Game/StarterContent/Materials/M_Brick_Clay_Beveled.M_Brick_Clay_Beveled")
      (Transformation|SetRelativeScale3D _staticmesh_2 "0.400000,0.400000,0.400000")
      (Transformation|AddLocalOffset _staticmesh_3 "0.000000,50.000000,0.000000" false false))
    (:NewEnumerator1
      (Components|StaticMesh|SetStaticMesh _staticmesh "/Game/StarterContent/Props/SM_Rock.SM_Rock")
      (Transformation|SetRelativeScale3D _staticmesh_2 "0.400000,0.400000,0.400000")
      (Transformation|AddLocalOffset _staticmesh_3 "0.000000,0.000000,0.000000" false false))
    (:NewEnumerator2
      (Components|StaticMesh|SetStaticMesh _staticmesh "/Game/StarterContent/Architecture/Pillar_50x500.Pillar_50x500")
      (Transformation|SetRelativeScale3D _staticmesh_2 "0.600000,0.600000,0.400000")
      (Transformation|AddLocalOffset _staticmesh_3 "0.000000,0.000000,0.000000" false false))
    (:NewEnumerator3
      (Components|StaticMesh|SetStaticMesh _staticmesh "/Game/StarterContent/Shapes/Shape_Pipe.Shape_Pipe")
      (Transformation|SetRelativeScale3D _staticmesh_2 "1.000000,1.000000,1.000000")
      (Transformation|AddLocalOffset _staticmesh_3 "0.000000,0.000000,70.000000" false false))
    (:NewEnumerator4
      (Components|StaticMesh|SetStaticMesh _staticmesh "/Game/StarterContent/Props/SM_Door.SM_Door")
      (Transformation|SetRelativeScale3D _staticmesh_2 "1.000000,1.000000,1.000000")
      (Transformation|AddLocalOffset _staticmesh_3 "0.000000,50.000000,0.000000" false false))))